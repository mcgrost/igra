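; BP_Igor is the player character, with axis movement, mouse look, jump, sprint and a toggle between two cameras.
; Movement input sets walk speed, allowing sprint only when started while moving forward and capping backward and strafe movement at walking speed.
; PlayerLoss ragdolls the mesh, calculates a score from Tick-accumulated time, then after a delay requests respawn from GM_OurGame and prints the score.
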(event `InputAction|Sprint`
  (params (Key :type "Key Structure"))
  ;[1 1 1] кнопка бігу
  (:`Pressed`
    (if (== (stale `InputAxis|MoveForvardBAck` AxisValue) 1.0)
      (set `self.isSprinting?` true)
      (else
        (set `self.isSprinting?` false))))
  (:`Released`
    (set `self.isSprinting?` false)))

(event `InputAction|ChangeCamera`
  (params (Key :type "Key Structure"))
  ;[1 1 1] зміна камери
  (:`Pressed`
    (`/Engine/EditorBlueprintResources/StandardMacros.FlipFlop`
      (:`A`
        (`ActorComponent.Deactivate` (`self.MainCamera`))
        (`ActorComponent.Activate` (`self.ExtraCamera`) false))
      (:`B`
        (`ActorComponent.Deactivate` (`self.ExtraCamera`))
        (`ActorComponent.Activate` (`self.MainCamera`) false)))))

(event `InputAxis|MoveForvardBAck`
  (params (AxisValue :type "Float (single-precision)"))
  (bind _charactermovement (`self.CharacterMovement`))
  ;[1 1 1] ходьба
  (`self.AddMovementInput` (`SceneComponent.GetForwardVector` (`self.CapsuleComponent`)) AxisValue)
  (`|ExecutionSequence`
    (:`then_0`
      ;[1 1 1] вперед
      (set `CharacterMovementComponent.MaxWalkSpeed` 201.0 _charactermovement))
    (:`then_1`
      ;[1 1 1] назад
      (if (== AxisValue -1.0)
        (set `CharacterMovementComponent.MaxWalkSpeed` 201.0 _charactermovement)))
    (:`then_2`
      ;[1 1 1] біг
      (if (`self.isSprinting?`)
        (set `CharacterMovementComponent.MaxWalkSpeed` 600.0 _charactermovement)))
    (:`then_3`
      ;[1 1 1] скорість стрейфа
      (if (`self.isWalkRightLeft`)
        (set `CharacterMovementComponent.MaxWalkSpeed` 201.0 (`self.CharacterMovement`))))
    (:`then_4`
      (if (== AxisValue -1.0)
        (set `CharacterMovementComponent.MaxWalkSpeed` 201.0 (`self.CharacterMovement`))))))

(event `InputAxis|LookUpDown`
  (params (AxisValue :type "Float (single-precision)"))
  ;[1 1 1] поворот мишкою
  (`self.AddControllerPitchInput` AxisValue))

(event `InputAxis|LookLestRight`
  (params (AxisValue :type "Float (single-precision)"))
  ;[1 1 1] поворот мишкою
  (`self.AddControllerYawInput` AxisValue))

(event `InputAxis|MoveRightLeft`
  (params (AxisValue :type "Float (single-precision)"))
  ;[1 1 1] ходьба
  (`self.AddMovementInput` (`SceneComponent.GetRightVector` (`self.CapsuleComponent`)) AxisValue)
  (set `self.isWalkRightLeft` (or (== AxisValue 1.0) (== AxisValue -1.0))))

(event `InputAction|Jump`
  (params (Key :type "Key Structure"))
  ;[1 1 1] прижок
  (:`Pressed`
    (`self.Jump`)))

(event `PlayerLoss`
  ;[1 1 1] подія програшу
  (`self.Dead`)
  (set `self.isLoss?` true)
  (`|ExecutionSequence`
    (:`then_0`
      (`KismetSystemLibrary.Delay` 3.0)
      (bind _asgm_our_game (cast `/Game/Level/GM_OurGame` (`GameplayStatics.GetGameMode`)))
      (`/Game/Level/GM_OurGame.Respawn` _asgm_our_game (`self.GetInstigatorController`))
      ;[1 1 1] вивід рахунка очків на екран
      (`KismetSystemLibrary.PrintText` (`KismetTextLibrary.Conv_DoubleToText` (`self.Score`) "HalfToEven")))
    (:`then_1`
      ;[1 1 1] розрахунок очків
      (if (`self.isLoss?`)
        (set `self.Score` (`KismetMathLibrary.Conv_IntToDouble` (`KismetMathLibrary.Round` (/ (`self.ElapsedTime`) 10.0))))))))

(event `self.ReceiveTick`
  (params (DeltaSeconds :type "Float (single-precision)"))
  ;[1 1 1] таймер для розрахунку очків
  (set `self.ElapsedTime` (+ DeltaSeconds (`self.ElapsedTime`))))

(fn `Dead`
  (`PrimitiveComponent.SetSimulatePhysics` (`self.Mesh`) true)
  (`CharacterMovementComponent.DisableMovement` (`self.CharacterMovement`)))

(fn `UserConstructionScript`)